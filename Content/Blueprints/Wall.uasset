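; Wall actor that toggles between a closed and an open position when its MoveWall event is called.
; The construction script records the actor's starting transform, and the open target is the Space transform converted from actor space.
; MoveComponentTo slides and rotates the static mesh between the two.
; After each move, it sets CanBePressed on the player's FPCharacter and flips the Open flag.
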(event `MoveWall`
  (bind _returnvalue (`self.GetTransform`))
  (bind _staticmeshcomponent (`self.StaticMeshComponent`))
  (bind (_space_location _space_rotation) (`KismetMathLibrary.BreakTransform` (`self.Space`)))
  (bind (_initialspace_location _initialspace_rotation) (`KismetMathLibrary.BreakTransform` (`self.InitialSpace`)))
  ;[1 1 1] Wall Movement
  (if (`self.Open?`)
    (`KismetSystemLibrary.MoveComponentTo` _staticmeshcomponent _initialspace_location _initialspace_rotation false false 1.0)
    (else
      (`KismetSystemLibrary.MoveComponentTo` _staticmeshcomponent (`KismetMathLibrary.TransformLocation` _returnvalue _space_location) (`KismetMathLibrary.TransformRotation` _returnvalue _space_rotation) false false 1.0)))
  (bind _asfpcharacter (cast `/Game/Blueprints/FPCharacter` (`GameplayStatics.GetPlayerPawn` 0)))
  (set `/Game/Blueprints/FPCharacter.canBePressed` true _asfpcharacter)
  (if (`self.Open?`)
    (set `self.Open?` false)
    (else
      (set `self.Open?` true))))

(fn `UserConstructionScript`
  (set `self.InitialSpace` (`KismetMathLibrary.MakeTransform` (`self.K2_GetActorLocation`) (`self.K2_GetActorRotation`))))